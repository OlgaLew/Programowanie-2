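; A floor-trigger reset button actor that checks crystal collection when the player overlaps its box.
; If no BP_Crystal actors remain in the level, the cube switches to a tech hex tile material; otherwise the player pawn teleports to a hardcoded location.
; Helper graphs for nudging the button down or up and briefly lighting it exist, but the overlap logic does not call them.
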(event `self.Box.OnComponentBeginOverlap`
  (params (OverlappedComponent :type "PrimitiveComponent Object Reference") (OtherActor :type "Actor Object Reference") (OtherComp :type "PrimitiveComponent Object Reference") (OtherBodyIndex :type Integer) (bFromSweep :type Boolean) (SweepResult :type "HitResult Structure (by ref)"))
  (`/Game/OlgaLewandowska/Blueprints/Actors/Libraries/ML_Actors.isPlayer` OtherActor
    (:`IsPlayer`
      (bind _outactors (`GameplayStatics.GetAllActorsOfClass` "/Game/OlgaLewandowska/Blueprints/Actors/BP_Crystal.BP_Crystal_C"))
      (if (== (`KismetArrayLibrary.Array_Length` _outactors) 0)
        (`PrimitiveComponent.SetMaterial` (`self.Cube`) 0 "/Game/StarterContent/Materials/M_Tech_Hex_Tile.M_Tech_Hex_Tile")
        (else
          (`self.K2_SetActorLocation` (`GameplayStatics.GetPlayerPawn` 0) (29.0 55.791763 -18.0) false false))))))

(fn `PushButton`
  (`self.K2_SetActorRelativeLocation` (- (`self.K2_GetActorLocation`) (0.0 0.0 4.0)) false true))

(fn `UpButton`
  (`self.K2_SetActorRelativeLocation` (+ (`self.K2_GetActorLocation`) (0.0 0.0 4.0)) false true))

(fn `UserConstructionScript`)