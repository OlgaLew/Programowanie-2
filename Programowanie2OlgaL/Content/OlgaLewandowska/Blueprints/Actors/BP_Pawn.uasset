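; Player pawn: a sphere rolled by physics torque from two input axes, scaled by a multiplier.
; On BeginPlay it records how many BP_Crystal actors the level holds and repositions the camera and spring arm for one level matched by name.
; Any damage kills it: the screen fades out, then the current level reopens slightly before the fade ends to avoid a bright flash.
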(event `self.ReceiveBeginPlay`
  (bind _outactors (`GameplayStatics.GetAllActorsOfClass` "/Game/OlgaLewandowska/Blueprints/Actors/BP_Crystal.BP_Crystal_C"))
  (set `self.HowMuchCrystalOnBeggining` (`KismetArrayLibrary.Array_Length` _outactors))
  (bind _returnvalue (`GameplayStatics.GetCurrentLevelName` true))
  (if (== (`KismetArrayLibrary.Array_Find` (`self.Name`) (`KismetStringLibrary.Conv_StringToName` _returnvalue)) 1)
    (`SceneComponent.K2_SetRelativeLocation` (`self.Camera`) (-200.0 0.0 0.0) false false)
    (`SceneComponent.K2_SetRelativeRotation` (`self.SpringArm`) (struct :`Pitch` -80.0) false false)))

(event `InputAxis|GoraDol`
  (params (AxisValue :type "Float (single-precision)"))
  (`PrimitiveComponent.AddTorqueInRadians` (`self.Sphere`) (`KismetMathLibrary.MakeVector` (* (stale `InputAxis|PrawoLewo` AxisValue) (`self.Mnozenie`)) (* AxisValue (`self.Mnozenie`))) "None" true :!label _label))

(event `InputAxis|PrawoLewo`
  (params (AxisValue :type "Float (single-precision)"))
  (goto _label))

(event `self.ReceiveAnyDamage`
  (params (Damage :type "Float (single-precision)") (DamageType :type "DamageType Object Reference") (InstigatedBy :type "Controller Object Reference") (DamageCauser :type "Actor Object Reference"))
  (`self.You Dead!`))

(fn `UserConstructionScript`)