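; BP_WinVolume is a level-exit volume that completes the level when the player overlaps its box with no BP_Crystal actors left in the world.
; If crystals remain, it only prints a debug string.
; On completion it finds the current level in a Name array, then opens the next entry by name or quits the game if it is the last.
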(event `self.Box.OnComponentBeginOverlap`
  (params (OverlappedComponent :type "PrimitiveComponent Object Reference") (OtherActor :type "Actor Object Reference") (OtherComp :type "PrimitiveComponent Object Reference") (OtherBodyIndex :type Integer) (bFromSweep :type Boolean) (SweepResult :type "HitResult Structure (by ref)"))
  (`/Game/OlgaLewandowska/Blueprints/Actors/Libraries/ML_Actors.isPlayer` OtherActor
    (:`IsPlayer`
      (if (`self.CheckAnyCrystals`)
        (`self.CompleteLevel`)
        (else
          (`KismetSystemLibrary.PrintString` "Crystals"))))))

(fn `CheckAnyCrystals`
  (returns (IsNoneCrystals :type Boolean))
  (bind _outactors (`GameplayStatics.GetAllActorsOfClass` "/Game/OlgaLewandowska/Blueprints/Actors/BP_Crystal.BP_Crystal_C"))
  (return (== (`KismetArrayLibrary.Array_Length` _outactors) 0)))

(fn `CompleteLevel`
  (bind _returnvalue (`GameplayStatics.GetCurrentLevelName` true))
  (if (`self.IsFinalLvl` (`self.GetCurrentLevelIndex` _returnvalue))
    (`KismetSystemLibrary.PrintString` "Last Level")
    (`KismetSystemLibrary.QuitGame` null "Quit")
    (return)
    (else
      (`KismetSystemLibrary.PrintString` "Not")
      (`self.LoadNextLevel`))))

(fn `GetCurrentLevelIndex`
  (params (InString :type String))
  (returns (IndeksNumer :type Integer))
  (return (`KismetArrayLibrary.Array_Find` (`self.Name`) (`KismetStringLibrary.Conv_StringToName` InString))))

(fn `GetNextLevelName`
  (params (Indexnumerinthislevel :type Integer))
  (returns (NextLevelName :type "Object Object Reference (by ref)"))
  (return (`|GetArrayItem` (`self.Name`) (+ Indexnumerinthislevel 1))))

(fn `IsFinalLvl`
  (params (`Index numer` :type Integer))
  (returns (IsLastLevel :type Boolean))
  (return (== `Index numer` (`KismetArrayLibrary.Array_LastIndex` (`self.Name`)))))

(fn `LoadNextLevel`
  (bind _returnvalue (`GameplayStatics.GetCurrentLevelName` true))
  (`GameplayStatics.OpenLevel` (`self.GetNextLevelName` (`self.GetCurrentLevelIndex` _returnvalue))))

(fn `UserConstructionScript`)