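; BP_lightbutton is a pressure button that temporarily switches on a spotlight when the player steps on it.
; A player overlapping the box drops the whole actor slightly and runs SetLight, which raises the spotlight intensity and zeroes it after a fixed delay.
; Any end overlap raises a pressed button again, independently of the light timer.
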(event `self.Box.OnComponentBeginOverlap`
  (params (OverlappedComponent :type "PrimitiveComponent Object Reference") (OtherActor :type "Actor Object Reference") (OtherComp :type "PrimitiveComponent Object Reference") (OtherBodyIndex :type Integer) (bFromSweep :type Boolean) (SweepResult :type "HitResult Structure (by ref)"))
  (`/Game/OlgaLewandowska/Blueprints/Actors/Libraries/ML_Actors.isPlayer` OtherActor
    (:`IsPlayer`
      (if (not (`self.IsPressed`))
        (`self.PushButton`)
        (set `self.IsPressed` true)
        (`self.SetLight`)))))

(event `self.Box.OnComponentEndOverlap`
  (params (OverlappedComponent :type "PrimitiveComponent Object Reference") (OtherActor :type "Actor Object Reference") (OtherComp :type "PrimitiveComponent Object Reference") (OtherBodyIndex :type Integer))
  (if (`self.IsPressed`)
    (`self.UpButton`)
    (set `self.IsPressed` false)))

(fn `PushButton`
  (`self.K2_SetActorRelativeLocation` (- (`self.K2_GetActorLocation`) (0.0 0.0 4.0)) false true))

(fn `UpButton`
  (`self.K2_SetActorRelativeLocation` (+ (`self.K2_GetActorLocation`) (0.0 0.0 4.0)) false true))

(fn `UserConstructionScript`)