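; BP_Crystal is a collectible crystal that rotates every tick and is picked up when the player pawn overlaps it.
; Pickup disables the box collision, stores the start location, then plays a timeline driving light intensity, scale and a lerp toward the player's current position.
; A DoOnce on the timeline's first update prints a one-coin message and destroys the actor after a short delay; no currency is stored here.
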(event `self.ReceiveTick`
  (params (DeltaSeconds :type "Float (single-precision)"))
  (`self.K2_AddActorWorldRotation` (struct :`Yaw` 1.0)))

(event `self.ReceiveActorBeginOverlap`
  (params (OtherActor :type "Actor Object Reference"))
  (`self.IsPlayer` OtherActor
    (:`IsPlayer`
      (`PrimitiveComponent.SetCollisionEnabled` (`self.Box`) "NoCollision")
      (`self.SetActorLocation`)
      (bind (_direction _lokacja _emisja _skala) (`Timeline|Timeline_0`)
        (:`Update`
          (`self.Swiatlo` _emisja)
          (`self.GetCrystalToActor` _lokacja)
          (`self.SetActorScale` _skala)
          (`/Engine/EditorBlueprintResources/StandardMacros.DoOnce` false
            (:`Completed`
              (`KismetSystemLibrary.PrintString` "1 moneta")
              (`KismetSystemLibrary.Delay` 0.5)
              (`self.K2_DestroyActor`))))))))

(fn `GetCrystalToActor`
  (params (Alpha :type "Float (double-precision)"))
  (`self.K2_SetActorLocation` (`KismetMathLibrary.VLerp` (`self.LerpStartLocation`) (`self.K2_GetActorLocation` (`GameplayStatics.GetPlayerPawn` 0)) Alpha)))

(fn `SetActorLocation`
  (set `self.LerpStartLocation` (`self.K2_GetActorLocation`)))

(fn `SetActorScale`
  (params (NewScale3D :type "Vector Structure") (`NewScale 2` :type "Float (double-precision)"))
  (`self.SetActorScale3D` NewScale3D))

(fn `Swiatlo`
  (params (NewIntensity :type "Float (double-precision)"))
  (`LightComponent.SetIntensity` (`self.PointLight`) NewIntensity))

(fn `UserConstructionScript`)