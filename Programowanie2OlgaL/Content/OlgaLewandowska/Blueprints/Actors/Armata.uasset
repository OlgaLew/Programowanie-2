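; Armata is a cannon actor that fires Pocisk1 projectiles automatically and repeatedly from BeginPlay.
; After a Pretkosc delay, it spawns a projectile at the Arrow's location and rotation, scaled by ProjectileScale.
; A timeline then moves the Cube1 barrel along relative Y, and its Cannon Fired event track loops back to the delay for the next shot.
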(event `self.ReceiveBeginPlay`
  (`KismetSystemLibrary.Delay` (`self.Pretkosc`) :!label _label)
  (`self.SpawnProjectile`)
  (bind (_direction _cannonbarrellocation) (`Timeline|Cannon Fire Timeline` :!via `PlayFromStart`)
    (:`Update`
      (`self.CannonBarrelY Location` _cannonbarrellocation))
    (:`Cannon Fired`
      (goto _label))))

(fn `CannonBarrelY Location`
  (params (NewLocation_Y :type "Float (double-precision)"))
  (`SceneComponent.K2_SetRelativeLocation` (`self.Cube1`) (`KismetMathLibrary.MakeVector` 0.0 NewLocation_Y) false false))

(fn `SpawnProjectile`
  (bind (_returnvalue_location _returnvalue_rotation) (`KismetMathLibrary.BreakTransform` (`SceneComponent.K2_GetComponentToWorld` (`self.Arrow`))))
  (`|SpawnActorFromClass` "/Game/OlgaLewandowska/Blueprints/Actors/Projectitles/Pocisk1.Pocisk1_C" (`KismetMathLibrary.MakeTransform` _returnvalue_location _returnvalue_rotation (`KismetMathLibrary.Conv_DoubleToVector` (`self.Projectile Scale`))) "Undefined" "OverrideRootScale" null null))

(fn `UserConstructionScript`)